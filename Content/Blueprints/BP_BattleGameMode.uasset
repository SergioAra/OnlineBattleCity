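; Battle game mode that spawns local multiplayer characters at the level's player starts after a short delay on BeginPlay.
; Each PlayerStart's tag is read as an integer serving as both player index and TeamId, with a local player created when that controller is missing.
; Each controller possesses its new BP_Character and switches its view to the shared BattleGameCameraActor, if one exists.
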(event `self.ReceiveBeginPlay`
  (bind _lastcontroller (`self.LastController`))
  (`KismetSystemLibrary.Delay` 5.0)
  (bind _outactors (`GameplayStatics.GetAllActorsOfClass` "/Script/Engine.PlayerStart"))
  (for _array_element _outactors
    (bind _returnvalue (`KismetStringLibrary.Conv_StringToInt` (`KismetStringLibrary.Conv_NameToString` (`PlayerStart.PlayerStartTag` _array_element))))
    (bind _returnvalue_2 (`GameplayStatics.GetPlayerController` _returnvalue))
    (if (`KismetSystemLibrary.IsValid` _returnvalue_2)
      (set `self.LastController` _returnvalue_2)
      (else
        (bind _returnvalue_3 (`GameplayStatics.CreatePlayer` -1))
        (set `self.LastController` _returnvalue_3)))
    (bind _returnvalue_4 (`|SpawnActorFromClass` "/Game/Blueprints/BP_Character.BP_Character_C" (`self.GetTransform` _array_element) "AdjustIfPossibleButAlwaysSpawn" "OverrideRootScale" null _returnvalue null))
    (`Controller.Possess` _lastcontroller _returnvalue_4)
    (bind _returnvalue_5 (`GameplayStatics.GetActorOfClass` "/Script/BattleCity.BattleGameCameraActor"))
    (`/Engine/EditorBlueprintResources/StandardMacros.IsValid` _returnvalue_5
      (:`Is Valid`
        (`PlayerController.SetViewTargetWithBlend` _lastcontroller _returnvalue_5 0.0 "VTBlend_Linear" 0.0 false)))))

(fn `UserConstructionScript`)